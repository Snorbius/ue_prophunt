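; Game mode for Prop Hunt that starts rounds, assigns hunter and hider roles, and tracks victory.
; A ready check gates game start, then one random player becomes a frozen hunter at the Hunter start and the rest become hiders at random Hider-tagged starts.
; Role changes go through player-state pawn swaps, including banishing hiders with death particles.
; UpdateNumberStatus recounts pawns by class into the game state and triggers victory when no hiders remain.
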(event `SwapToHunter`
  (params (PlayerState :type "/Game/PropHunt/Core/BP_PropHuntPlayerState Object Reference"))
  (`/Game/PropHunt/Core/BP_PropHuntPlayerState.SwapControlledPawn` PlayerState "NewEnumerator2")
  (`self.K2_SetActorTransform` (`PlayerState.GetPawn` PlayerState) (`self.GetTransform` (`self.K2_FindPlayerStart` (`PlayerState.GetPlayerController` PlayerState) "Hunter")) false false)
  (`self.UpdateNumberStatus`))

(event `self.K2_OnLogout`
  (params (ExitingController :type "Controller Object Reference"))
  (`self.UpdateNumberStatus`))

(event `self.ReceiveBeginPlay`
  (bind _asbp_prop_hunt_game_state (cast `/Game/PropHunt/Core/BP_PropHuntGameState` (`GameplayStatics.GetGameState`)))
  (set `self.GameStateRef` _asbp_prop_hunt_game_state))

(event `BanishHider`
  (params (Hider :type "/Game/PropHunt/Core/BP_Hider Object Reference"))
  (bind _asbp_prop_hunt_player_state (cast `/Game/PropHunt/Core/BP_PropHuntPlayerState` (`Pawn.PlayerState` Hider)))
  (`/Game/PropHunt/Core/BP_PropHuntPlayerState.Multicast_SpawnHiderDeathParticles` _asbp_prop_hunt_player_state (`self.K2_GetActorLocation` Hider))
  (`/Game/PropHunt/Core/BP_PropHuntPlayerState.SwapControlledPawn` _asbp_prop_hunt_player_state "NewEnumerator0")
  (`self.UpdateNumberStatus`))

(event `BeginGame`
  (`KismetSystemLibrary.PrintString` "Begin game!!!" :!label _label)
  (`/Game/PropHunt/Core/BP_PropHuntGameState.StartGame` (`self.GameStateRef`))
  (`self.InitializePlayers`))

(event `AttemptBeginGame`
  (`self.CanBegin`
    (:`true`
      (goto _label))
    (:`false`
      (`KismetSystemLibrary.PrintString` "Couldn't start game"))))

(event `self.K2_PostLogin`
  (params (NewPlayer :type "PlayerController Object Reference"))
  (bind _asbp_prop_hunt_controller (cast `/Game/PropHunt/Core/BP_PropHuntController` NewPlayer))
  (`/Game/PropHunt/Core/BP_PropHuntController.SetInputMode` _asbp_prop_hunt_controller true))

(fn `CanBeginFunction`
  (returns (success :type Boolean))
  (for _index (range (`GameplayStatics.GetNumPlayerStates`))
    (bind _asbp_prop_hunt_player_state (cast `/Game/PropHunt/Core/BP_PropHuntPlayerState` (`GameplayStatics.GetPlayerState` _index)))
    (if (not (`/Game/PropHunt/Core/BP_PropHuntPlayerState.IsReady` _asbp_prop_hunt_player_state))
      (return false)))
  (return true))

(fn `CheckReadyState`
  (for _index (range (`GameplayStatics.GetNumPlayerStates`))
    (bind _asbp_prop_hunt_player_state (cast `/Game/PropHunt/Core/BP_PropHuntPlayerState` (`GameplayStatics.GetPlayerState` _index)))
    (if (not (`/Game/PropHunt/Core/BP_PropHuntPlayerState.IsReady` _asbp_prop_hunt_player_state))
      (`self.OnAnyoneNotReady`)
      (return)))
  (`self.OnEveryoneReady`))

(fn `CheckVictory`
  (bind _outactors (`GameplayStatics.GetAllActorsOfClass` "/Game/PropHunt/Core/BP_Hider.BP_Hider_C"))
  (if (`KismetArrayLibrary.Array_IsEmpty` _outactors)
    (`/Game/PropHunt/Core/BP_PropHuntGameState.Multicast_CallVictory` (`self.GameStateRef`))))

(fn `GetAvailableHiderSpawns`
  (returns (out :type "Array of PlayerStart Object Reference"))
  (locals (res :type "Array of PlayerStart Object Reference"))
  (bind _outactors (`GameplayStatics.GetAllActorsOfClass` "/Script/Engine.PlayerStart"))
  (for _array_element _outactors
    (if (== (`PlayerStart.PlayerStartTag` _array_element) "Hider")
      (`KismetArrayLibrary.Array_Add` (`local.res`) _array_element)))
  (return (`local.res`)))

(fn `GetPlayerStates`
  (returns (Out :type "Array of /Game/PropHunt/Core/BP_PropHuntPlayerState Object Reference"))
  (locals (Res :type "Array of /Game/PropHunt/Core/BP_PropHuntPlayerState Object Reference"))
  (for _index (range (`GameplayStatics.GetNumPlayerStates`))
    (bind _asbp_prop_hunt_player_state (cast `/Game/PropHunt/Core/BP_PropHuntPlayerState` (`GameplayStatics.GetPlayerState` _index)))
    (`KismetArrayLibrary.Array_Add` (`local.Res`) _asbp_prop_hunt_player_state))
  (return (`local.Res`)))

(fn `InitializePlayers`
  (locals (PlayerStates :type "Array of /Game/PropHunt/Core/BP_PropHuntPlayerState Object Reference") (HunterPlayerState :type "/Game/PropHunt/Core/BP_PropHuntPlayerState Object Reference"))
  (bind _out (`self.GetPlayerStates`))
  (set `local.PlayerStates` _out)
  (`|ExecutionSequence`
    (:`then_0`
      (bind _output_get (set `local.HunterPlayerState` (`KismetArrayLibrary.Array_Random` (`local.PlayerStates`))))
      (`KismetArrayLibrary.Array_RemoveItem` (`local.PlayerStates`) _output_get)
      (`/Game/PropHunt/Core/BP_PropHuntPlayerState.SwapControlledPawn` _output_get "NewEnumerator2")
      (bind _returnvalue (`PlayerState.GetPawn` _output_get))
      (`self.K2_SetActorTransform` _returnvalue (`self.GetTransform` (`self.K2_FindPlayerStart` (`PlayerState.GetPlayerController` _output_get) "Hunter")) false false)
      (`/Game/PropHunt/Core/BP_PropHuntPlayerState.SetControlRotation` _output_get (`self.K2_GetActorRotation` _returnvalue))
      (bind _asbp_hunter (cast `/Game/PropHunt/Core/BP_Hunter` (`PlayerState.GetPawn` (`local.HunterPlayerState`))))
      (`/Game/PropHunt/Core/BP_Hunter.FreezeHunter` _asbp_hunter (`self.HunterFreezeTime`)))
    (:`then_1`
      (bind _out_2 (`self.GetAvailableHiderSpawns`))
      (for _array_element (`local.PlayerStates`)
        (`/Game/PropHunt/Core/BP_PropHuntPlayerState.SwapControlledPawn` _array_element "NewEnumerator1")
        (bind _returnvalue_2 (`PlayerState.GetPawn` _array_element))
        (`self.K2_SetActorTransform` _returnvalue_2 (`self.GetTransform` (`KismetArrayLibrary.Array_Random` _out_2)) false false)
        (`/Game/PropHunt/Core/BP_PropHuntPlayerState.SetControlRotation` _array_element (`self.K2_GetActorRotation` _returnvalue_2))))
    (:`then_2`
      (`self.UpdateNumberStatus`))))

(fn `UpdateNumberStatus`
  ; Very ugly way of doing this but it gives me an easy function to call in every relevant scenario (hider death, spectator convert, player join, player leave etc.)
  (bind _outactors (`GameplayStatics.GetAllActorsOfClass` "/Game/PropHunt/Core/BP_Hunter.BP_Hunter_C"))
  (set `/Game/PropHunt/Core/BP_PropHuntGameState.NumHunters` (`KismetArrayLibrary.Array_Length` _outactors) (`self.GameStateRef`))
  (bind _outactors_2 (`GameplayStatics.GetAllActorsOfClass` "/Game/PropHunt/Core/BP_Hider.BP_Hider_C"))
  (set `/Game/PropHunt/Core/BP_PropHuntGameState.NumHiders` (`KismetArrayLibrary.Array_Length` _outactors_2) (`self.GameStateRef`))
  (`self.CheckVictory`))

(fn `UserConstructionScript`)