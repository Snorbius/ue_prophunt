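; Prop Hunt game instance that handles online sessions: hosting a listen server on the dungeon map, quick join, session search, invites and quitting to the menu.
; Hosting, joining and quitting first destroy any existing session, then proceed regardless of the result.
; DoOnce gates block overlapping searches, with dispatchers reporting browser search results.
; Quick join filters on ServerValidateKey as a bool, hosting sets it as a string, and browser search is unfiltered.
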(event `HostGame`
  (bind _returnvalue (`GameplayStatics.GetPlayerController` 0))
  (`DestroySessionCallbackProxy.DestroySession` _returnvalue
    (:`OnSuccess`
      _)
    (:`OnFailure`
      _))
  (`CreateSessionCallbackProxyAdvanced.CreateAdvancedSession` (`|MakeArray` (`AdvancedSessionsLibrary.MakeLiteralSessionPropertyString` (`self.ServerValidateKey`) "true")) _returnvalue 24
    (:`OnSuccess`
      (`GameplayStatics.OpenLevelBySoftObjectPtr` "/Game/PropHunt/Levels/LVL_Dungeon1.LVL_Dungeon1" true "listen"))))

(event `QuitToMenu`
  (`DestroySessionCallbackProxy.DestroySession` (`GameplayStatics.GetPlayerController` 0)
    (:`OnSuccess`
      _)
    (:`OnFailure`
      _))
  (`GameplayStatics.OpenLevelBySoftObjectPtr` "/Game/PropHunt/Levels/LVL_Menu.LVL_Menu"))

(event `self.OnSessionInviteAccepted`
  (params (LocalPlayerNum :type Integer) (PersonInvited :type "BPUniqueNetId Structure") (SessionToJoin :type "BlueprintSessionResult Structure (by ref)"))
  (`self.JoinSpecificSession` SessionToJoin))

(event `QuickJoin`
  (`/Engine/EditorBlueprintResources/StandardMacros.DoOnce` false :!label _label
    (:`Completed`
      (`KismetSystemLibrary.PrintString` "Quick joining session..." true true (struct :`G` 0.66 :`B` 1.0 :`A` 1.0) 3.0)
      (bind _results (`FindSessionsCallbackProxyAdvanced.FindSessionsAdvanced` (`GameplayStatics.GetPlayerController` 0) 1 false "AllServers" (`|MakeArray` (`AdvancedSessionsLibrary.MakeLiteralSessionSearchProperty` (`AdvancedSessionsLibrary.MakeLiteralSessionPropertyBool` (`self.ServerValidateKey`) true) "Equals")))
        (:`OnSuccess`
          (if (`KismetArrayLibrary.Array_IsNotEmpty` _results)
            (`KismetSystemLibrary.PrintString` "Found session!" true true (struct :`G` 0.66 :`B` 1.0 :`A` 1.0) 3.0)
            (`self.JoinSpecificSession` (`|GetArrayItem` _results))
            (goto _label :!via `Reset`)
            (else
              _)))
        (:`OnFailure`
          _))
      (`KismetSystemLibrary.PrintString` "Could not find any sessions..." true true (struct :`G` 0.66 :`B` 1.0 :`A` 1.0) 3.0)
      (goto _label :!via `Reset`))))

(event `JoinSpecificSession`
  (params (Session :type "BlueprintSessionResult Structure (by ref)"))
  (bind _returnvalue (`GameplayStatics.GetPlayerController` 0))
  (`DestroySessionCallbackProxy.DestroySession` _returnvalue
    (:`OnSuccess`
      _)
    (:`OnFailure`
      _))
  (`JoinSessionCallbackProxy.JoinSession` _returnvalue Session
    (:`OnSuccess`
      (`KismetSystemLibrary.PrintString` "Joined Session!" true true (struct :`G` 0.66 :`B` 1.0 :`A` 1.0) 3.0))
    (:`OnFailure`
      (`KismetSystemLibrary.PrintString` "Failed to join session..." true true (struct :`G` 0.66 :`B` 1.0 :`A` 1.0) 3.0))))

(event `FetchAvailableSessions`
  (`/Engine/EditorBlueprintResources/StandardMacros.DoOnce` false :!label _label_2
    (:`Completed`
      (`self.OnBeginSearchForSessions`)
      (`KismetSystemLibrary.PrintString` "Finding available sessions..." true true (struct :`G` 0.66 :`B` 1.0 :`A` 1.0) 3.0)
      (bind _results (`FindSessionsCallbackProxyAdvanced.FindSessionsAdvanced` (`GameplayStatics.GetPlayerController` 0) 10 false "AllServers")
        (:`OnSuccess`
          (if (`KismetArrayLibrary.Array_IsNotEmpty` _results)
            (set `self.LastSessionFetchResult` _results)
            (`KismetSystemLibrary.PrintText` (`|FormatText` "Found {num} sessions!" (`KismetArrayLibrary.Array_Length` _results)))
            (`self.OnSessionsFound` (`self.LastSessionFetchResult`))
            (goto _label_2 :!via `Reset`)
            (else
              _)))
        (:`OnFailure`
          _))
      (`KismetSystemLibrary.PrintString` "Failed to find any sessions..." true true (struct :`G` 0.66 :`B` 1.0 :`A` 1.0) 3.0)
      (`self.OnNoSessionsFound`)
      (goto _label_2 :!via `Reset`))))

(fn `GetCoreActors`
  (returns (`AsGM Prop Hunt` :type "/Game/PropHunt/Core/GM_PropHunt Object Reference") (`AsBP Prop Hunt Game State` :type "/Game/PropHunt/Core/BP_PropHuntGameState Object Reference") (`AsBP Prop Hunt Game Instance` :type "/Game/PropHunt/Core/BP_PropHuntGameInstance Object Reference") (`AsBP Prop Hunt Controller` :type "/Game/PropHunt/Core/BP_PropHuntController Object Reference"))
  (bind _asgm_prop_hunt (cast `/Game/PropHunt/Core/GM_PropHunt` (`GameplayStatics.GetGameMode`))
    (:`then`
      _)
    (:`CastFailed`
      _))
  (bind _asbp_prop_hunt_game_state (cast `/Game/PropHunt/Core/BP_PropHuntGameState` (`GameplayStatics.GetGameState`))
    (:`then`
      _)
    (:`CastFailed`
      _))
  (bind _asbp_prop_hunt_game_instance (cast `/Game/PropHunt/Core/BP_PropHuntGameInstance` (`GameplayStatics.GetGameInstance`))
    (:`then`
      _)
    (:`CastFailed`
      _))
  (bind _asbp_prop_hunt_controller (cast `/Game/PropHunt/Core/BP_PropHuntController` (`GameplayStatics.GetPlayerController` 0))
    (:`then`
      _)
    (:`CastFailed`
      _))
  (return _asgm_prop_hunt _asbp_prop_hunt_game_state _asbp_prop_hunt_game_instance _asbp_prop_hunt_controller))