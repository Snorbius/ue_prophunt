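; Game state for a prop hunt mode that tracks whether a match is running and how many hunters and hiders there are.
; StartGame runs on authority and multicasts the start, setting IsGameStarted and firing OnGameStart, while a victory multicast clears the flag and fires OnVictory.
; RepNotify handlers on the hunter and hider counts rebroadcast changes through event dispatchers.
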(event `StartGame`
  (`/Engine/EditorBlueprintResources/ActorMacros.Switch Has Authority`
    (:`Authority`
      (`self.Multicast_StartGame`)
      (set `self.IsGameStarted` true))))

(event `Multicast_StartGame`
  (`self.OnGameStart`)
  (`KismetSystemLibrary.PrintString` "Game is starting!!")
  (set `self.IsGameStarted` true))

(event `Multicast_CallVictory`
  (`self.Victory`))

(fn `OnRep_NumHiders`
  (`self.OnNumHidersChange` (`self.NumHiders`)))

(fn `OnRep_NumHunters`
  (`self.OnNumHuntersChanged` (`self.NumHunters`)))

(fn `UserConstructionScript`)

(fn `Victory`
  (set `self.IsGameStarted` false)
  (`self.OnVictory`))