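; Free-flying spectator pawn for Prop Hunt that can betray the hiders by asking the game mode to swap it to a hunter mid-game.
; Camera-relative input drives a FloatingPawnMovement, with horizontal motion flattened and a separate vertical axis.
; Custom movement sync has the locally controlled pawn send its transform to the server each tick, while non-local copies lerp toward SyncTransform.
; Game state start and victory events control the spectator UI's visibility.
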(event `self.ReceiveBeginPlay`
  (set `self.SyncTransform` (`self.GetTransform`))
  (bind _returnvalue (`|CreateWidget` "/Game/PropHunt/Blueprints/UI/WBP_SpectatorUI.WBP_SpectatorUI_C"))
  (bind _output_get (set `self.SpectatorUI` _returnvalue))
  (`UserWidget.AddToViewport` _output_get 0)
  (bind _asbp_prop_hunt_game_state (cast `/Game/PropHunt/Core/BP_PropHuntGameState` (`GameplayStatics.GetGameState`)))
  (set `self.GameStateRef` _asbp_prop_hunt_game_state)
  (set `Widget.Visibility` (select `bool` (`/Game/PropHunt/Core/BP_PropHuntGameState.IsGameStarted` _asbp_prop_hunt_game_state) :`false` "Hidden" :`true` "Visible" :!type "ESlateVisibility Enum") (`self.SpectatorUI`))
  (add `/Game/PropHunt/Core/BP_PropHuntGameState.OnGameStart` _asbp_prop_hunt_game_state (`|CreateDelegate` :!event `OnGameStart`))
  (add `/Game/PropHunt/Core/BP_PropHuntGameState.OnVictory` _asbp_prop_hunt_game_state (`|CreateDelegate` :!event `OnGameEnd`)))

(event `EnhancedInput|/Game/PropHunt/Input/Actions/IA_Move`
  (params (ActionValue :type "Vector Structure") (ElapsedSeconds :type "Float (double-precision)") (TriggeredSeconds :type "Float (double-precision)") (InputAction :type "InputAction Object Reference" :default "/Game/PropHunt/Input/Actions/IA_Move.IA_Move"))
  (bind _floatingpawnmovement (`self.FloatingPawnMovement`))
  (bind _camera (`self.Camera`))
  (:`Triggered`
    (`PawnMovementComponent.AddInputVector` _floatingpawnmovement (* (.x ActionValue) (`KismetMathLibrary.Normal` (`KismetMathLibrary.MakeVector` (.x (`SceneComponent.GetRightVector` _camera)) (.y (`SceneComponent.GetRightVector` _camera))))) false)
    (`PawnMovementComponent.AddInputVector` _floatingpawnmovement (* (.y ActionValue) (`KismetMathLibrary.Normal` (`KismetMathLibrary.MakeVector` (.x (`SceneComponent.GetForwardVector` _camera)) (.y (`SceneComponent.GetForwardVector` _camera))))) false)
    (`PawnMovementComponent.AddInputVector` _floatingpawnmovement (* (.z ActionValue) (0.0 0.0 1.0)) false)))

(event `EnhancedInput|/Game/PropHunt/Input/Actions/IA_BetrayHiders`
  (params (ActionValue :type Boolean) (ElapsedSeconds :type "Float (double-precision)") (TriggeredSeconds :type "Float (double-precision)") (InputAction :type "InputAction Object Reference" :default "/Game/PropHunt/Input/Actions/IA_BetrayHiders.IA_BetrayHiders"))
  (:`Started`
    (if (`/Game/PropHunt/Core/BP_PropHuntGameState.IsGameStarted` (`self.GameStateRef`))
      (`self.Server_SwapSelfToHunter`))))

(event `EnhancedInput|/Game/PropHunt/Input/Actions/IA_Look`
  (params (ActionValue :type "Vector2D Structure") (ElapsedSeconds :type "Float (double-precision)") (TriggeredSeconds :type "Float (double-precision)") (InputAction :type "InputAction Object Reference" :default "/Game/PropHunt/Input/Actions/IA_Look.IA_Look"))
  (bind (_x _y) (`KismetMathLibrary.BreakVector2D` ActionValue))
  (:`Triggered`
    (`self.AddControllerYawInput` _x)
    (`self.AddControllerPitchInput` (* _y -1.0))))

(event `Server_SwapSelfToHunter`
  (bind _asgm_prop_hunt (cast `/Game/PropHunt/Core/GM_PropHunt` (`GameplayStatics.GetGameMode`)))
  (bind _asbp_prop_hunt_player_state (cast `/Game/PropHunt/Core/BP_PropHuntPlayerState` (`self.PlayerState`)))
  (`/Game/PropHunt/Core/GM_PropHunt.SwapToHunter` _asgm_prop_hunt _asbp_prop_hunt_player_state))

(event `self.ReceiveTick`
  (params (DeltaSeconds :type "Float (single-precision)"))
  (if (`self.IsLocallyControlled`)
    (`self.Server_UpdateSyncTransform` (`self.GetTransform`))
    (else
      (`self.K2_SetActorTransform` (`KismetMathLibrary.TLerp` (`self.GetTransform`) (`self.SyncTransform`) (`KismetMathLibrary.FMin` (* DeltaSeconds (`self.SyncStrength`)) 1.0))))))

(event `self.ReceiveEndPlay`
  (params (EndPlayReason :type "EEndPlayReason Enum" :default "Destroyed"))
  (`Widget.RemoveFromParent` (`self.SpectatorUI`)))

(event `Server_UpdateSyncTransform`
  (params (SyncTransform :type "Transform Structure"))
  (set `self.SyncTransform` SyncTransform))

(event `OnGameStart`
  (set `Widget.Visibility` "Visible" (`self.SpectatorUI`)))

(event `OnGameEnd`
  (set `Widget.Visibility` "Hidden" (`self.SpectatorUI`)))

(fn `UserConstructionScript`)