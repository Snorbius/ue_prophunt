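; Base character Blueprint for PropHunt that turns Enhanced Input actions into movement, camera look and jumping.
; IA_Move and IA_Look pass their axis values to Move and Aim functions defined outside these graphs, with the look Y axis inverted.
; IA_Jump starts a jump on Started and stops it on Canceled or Completed.
; The construction script only calls its parent.
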(event `EnhancedInput|/Game/PropHunt/Input/Actions/IA_Move`
  (params (ActionValue :type "Vector Structure") (ElapsedSeconds :type "Float (double-precision)") (TriggeredSeconds :type "Float (double-precision)") (InputAction :type "InputAction Object Reference" :default "/Game/PropHunt/Input/Actions/IA_Move.IA_Move"))
  (:`Triggered`
    (`self.Move` (.x ActionValue) (.y ActionValue))))

(event `EnhancedInput|/Game/PropHunt/Input/Actions/IA_Look`
  (params (ActionValue :type "Vector2D Structure") (ElapsedSeconds :type "Float (double-precision)") (TriggeredSeconds :type "Float (double-precision)") (InputAction :type "InputAction Object Reference" :default "/Game/PropHunt/Input/Actions/IA_Look.IA_Look"))
  (bind (_x _y) (`KismetMathLibrary.BreakVector2D` ActionValue))
  (:`Triggered`
    (`self.Aim` _x (* _y -1.0))))

(event `EnhancedInput|/Game/PropHunt/Input/Actions/IA_Jump`
  (params (ActionValue :type Boolean) (ElapsedSeconds :type "Float (double-precision)") (TriggeredSeconds :type "Float (double-precision)") (InputAction :type "InputAction Object Reference" :default "/Game/PropHunt/Input/Actions/IA_Jump.IA_Jump"))
  (:`Started`
    (`self.Jump`))
  (:`Canceled`
    (`self.StopJumping` :!label _label))
  (:`Completed`
    (goto _label)))

(fn `UserConstructionScript`
  (`parent.UserConstructionScript`))