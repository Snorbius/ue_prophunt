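; Hunter character for the Prop Hunt mode, able to shoot hiders and toggle between third and first person.
; A timed round-start freeze disables movement and fades the local screen dark through a post-process cover material.
; Firing runs a server-side sphere trace with debug drawing, and hits on BP_Hider are passed to GM_PropHunt to banish.
; The view toggle tweens boom length, switching yaw control and owner mesh visibility.
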(event `Client_Darken`
  (bind (_handle _currentvalue) (`|TweenFloat` (make `TweenFloatSettings` 0.0 1.0 (make `TweenSettings` (`self.CameraCoverFadeTime`) "InQuad" (struct :`EditorCurveData` (struct :`Keys` "((),(Time=1.000000,Value=1.000000))" :`DefaultValue` 3.4028234663852886e+38 :`PreInfinityExtrap` "RCCE_Constant" :`PostInfinityExtrap` "RCCE_Constant")) 0 "Restart" (make `TweenDelays` 0.0))))
    (:`OnUpdate`
      (`MaterialInstanceDynamic.SetScalarParameterValue` (`self.CoverMaterial`) "Opacity" _currentvalue))))

(event `Client_Lighten`
  (bind (_handle _currentvalue) (`|TweenFloat` (make `TweenFloatSettings` 1.0 0.0 (make `TweenSettings` (`self.CameraCoverFadeTime`) "InQuad" (struct :`EditorCurveData` (struct :`Keys` "((),(Time=1.000000,Value=1.000000))" :`DefaultValue` 3.4028234663852886e+38 :`PreInfinityExtrap` "RCCE_Constant" :`PostInfinityExtrap` "RCCE_Constant")) 0 "Restart" (make `TweenDelays` 0.0))))
    (:`OnUpdate`
      (`MaterialInstanceDynamic.SetScalarParameterValue` (`self.CoverMaterial`) "Opacity" _currentvalue))))

(event `DisableHunter`
  ; Freeze hunter at start of round
  (`CharacterMovementComponent.DisableMovement` (`self.CharacterMovement`))
  (`self.Client_Darken`))

(event `EnableHunter`
  ; Freeze hunter at start of round
  (`CharacterMovementComponent.SetMovementMode` (`self.CharacterMovement`) "MOVE_Walking" 0)
  (`self.Client_Lighten`))

(event `FreezeHunter`
  (params (Duration :type "Float (double-precision)"))
  ; Freeze hunter at start of round
  (`self.DisableHunter`)
  (bind _returnvalue (`KismetSystemLibrary.K2_SetTimerDelegate` (`|CreateDelegate` :!event `EnableHunter`) Duration))
  (set `self.FreezeHunterTimerHandle` _returnvalue))

(event `ClearFreezeTimer`
  (bind _freezehuntertimerhandle (`self.FreezeHunterTimerHandle`))
  ; Clears the timer (in case round is restarted while hunter is still frozen or otherwise)
  (if (`KismetSystemLibrary.K2_IsTimerActiveHandle` _freezehuntertimerhandle)
    (`KismetSystemLibrary.K2_ClearAndInvalidateTimerHandle` _freezehuntertimerhandle)))

(event `Server_ShootGun`
  (bind (_start _end) (`self.GetGunTraceLocations`))
  ; These two are seperate because I initially wanted to get the locations on the client for better responsiveness
  (bind _outhit (`self.GunTrace` _start _end)
    (:`hit`
      (bind _hider (`self.ValidateHit` _outhit)
        (:`PlayerHit`
          (`/Engine/EditorBlueprintResources/ActorMacros.Switch Has Authority`
            (:`Authority`
              (bind _asgm_prop_hunt (cast `/Game/PropHunt/Core/GM_PropHunt` (`GameplayStatics.GetGameMode`)))
              (`/Game/PropHunt/Core/GM_PropHunt.BanishHider` _asgm_prop_hunt _hider))))))))

(event `EnhancedInput|/Game/PropHunt/Input/Actions/IA_FireGun`
  (params (ActionValue :type Boolean) (ElapsedSeconds :type "Float (double-precision)") (TriggeredSeconds :type "Float (double-precision)") (InputAction :type "InputAction Object Reference" :default "/Game/PropHunt/Input/Actions/IA_FireGun.IA_FireGun"))
  (:`Started`
    (`self.Server_ShootGun`)))

(event `EnhancedInput|/Game/PropHunt/Input/Actions/IA_ToggleFirstPerson`
  (params (ActionValue :type Boolean) (ElapsedSeconds :type "Float (double-precision)") (TriggeredSeconds :type "Float (double-precision)") (InputAction :type "InputAction Object Reference" :default "/Game/PropHunt/Input/Actions/IA_ToggleFirstPerson.IA_ToggleFirstPerson"))
  (:`Started`
    (`/Engine/EditorBlueprintResources/StandardMacros.DoOnce` false :!label _label
      (:`Completed`
        (bind _isa (`/Engine/EditorBlueprintResources/StandardMacros.FlipFlop`)
          (:`A`
            _)
          (:`B`
            (set `self.bUseControllerRotationYaw` false)
            (`PrimitiveComponent.SetOwnerNoSee` (`self.Mesh`) false)))
        (bind (_handle _currentvalue) (`|TweenFloat` (make `TweenFloatSettings` (`SpringArmComponent.TargetArmLength` (`self.CameraBoom`)) (`KismetMathLibrary.SelectFloat` 0.0 400.0 _isa) (make `TweenSettings` 0.75 "InOutSine" (struct :`EditorCurveData` (struct :`Keys` "((),(Time=1.000000,Value=1.000000))" :`DefaultValue` 3.4028234663852886e+38 :`PreInfinityExtrap` "RCCE_Constant" :`PostInfinityExtrap` "RCCE_Constant")) 0 "Restart" (make `TweenDelays` 0.0))))
          (:`OnUpdate`
            (set `SpringArmComponent.TargetArmLength` _currentvalue (`self.CameraBoom`)))
          (:`OnComplete`
            (bind _output_get (set `self.bUseControllerRotationYaw` _isa))
            (`PrimitiveComponent.SetOwnerNoSee` (`self.Mesh`) _output_get)
            (goto _label :!via `Reset`)))))))

(fn `UserConstructionScript`
  (`parent.UserConstructionScript`)
  (if (`self.IsLocallyControlled`)
    (bind _returnvalue (`KismetMaterialLibrary.CreateDynamicMaterialInstance` "/Game/PropHunt/Art/Materials/M_CameraCover.M_CameraCover"))
    (bind _output_get (set `self.CoverMaterial` _returnvalue))
    (setmembers `PostProcessSettings` :`StructRef` (`CameraComponent.PostProcessSettings` (`self.FollowCamera`)) :`WeightedBlendables` (make `WeightedBlendables` (`|MakeArray` (make `WeightedBlendable` 1.0 _output_get))))))