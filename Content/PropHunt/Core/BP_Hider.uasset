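; Player character for Prop Hunt hiders, who disguise themselves as nearby props and can lock their rotation.
; A camera-directed sphere trace finds props; scroll input cycles the hits and an overlay material highlights the selection locally.
; SwapMesh flip-flops two mesh components, tweening one's scale out and then the other's in.
; Swaps and rotation locks apply locally first, then replicate through server RPCs and multicasts that skip the local controller.
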(event `Multicast_SetRotationLock`
  (params (Value :type Boolean) (LastRotation :type "Rotator Structure"))
  ; Rotation Lock
  (if (not (`self.IsLocallyControlled`))
    (set `CharacterMovementComponent.bOrientRotationToMovement` Value (`self.CharacterMovement`))
    (`SceneComponent.K2_SetWorldRotation` (`self.CapsuleComponent`) LastRotation false false)))

(event `Multicast_SwapMesh`
  (params (NewMesh :type "StaticMesh Object Reference"))
  ; Swap Mesh
  (if (not (`self.IsLocallyControlled`))
    (`self.SwapMesh` NewMesh)))

(event `Server_SetRotationLock`
  (params (Value :type Boolean) (LastRotation :type "Rotator Structure"))
  ; Rotation Lock
  (`self.Multicast_SetRotationLock` Value LastRotation))

(event `Server_SwapMesh`
  (params (NewMesh :type "StaticMesh Object Reference"))
  ; Swap Mesh
  (`self.Multicast_SwapMesh` NewMesh))

(event `EnhancedInput|/Game/PropHunt/Input/Actions/IA_ToggleRotationLock`
  (params (ActionValue :type Boolean) (ElapsedSeconds :type "Float (double-precision)") (TriggeredSeconds :type "Float (double-precision)") (InputAction :type "InputAction Object Reference" :default "/Game/PropHunt/Input/Actions/IA_ToggleRotationLock.IA_ToggleRotationLock"))
  (bind _charactermovement (`self.CharacterMovement`))
  ; Rotation Lock
  (:`Started`
    (bind _output_get (set `CharacterMovementComponent.bOrientRotationToMovement` (not (`CharacterMovementComponent.bOrientRotationToMovement` _charactermovement)) _charactermovement))
    (`self.Server_SetRotationLock` _output_get (`SceneComponent.K2_GetComponentRotation` (`self.CapsuleComponent`)))))

(event `EnhancedInput|/Game/PropHunt/Input/Actions/IA_SwapMesh`
  (params (ActionValue :type Boolean) (ElapsedSeconds :type "Float (double-precision)") (TriggeredSeconds :type "Float (double-precision)") (InputAction :type "InputAction Object Reference" :default "/Game/PropHunt/Input/Actions/IA_SwapMesh.IA_SwapMesh"))
  ; Swap Mesh
  (:`Started`
    (bind _asstatic_mesh_component (`self.GetPotentialMesh`)
      (:`true`
        (`/Engine/EditorBlueprintResources/StandardMacros.DoOnce` false :!label _label
          (:`Completed`
            (bind _staticmesh (`StaticMeshComponent.StaticMesh` _asstatic_mesh_component))
            (`self.SwapMesh` _staticmesh
              (:`then`
                (`self.Server_SwapMesh` _staticmesh))
              (:`On Complete`
                (goto _label :!via `Reset`)))))))))

(event `self.ReceiveTick`
  (params (DeltaSeconds :type "Float (single-precision)"))
  (`self.HighlightPotentialMesh`))

(event `EnhancedInput|/Game/PropHunt/Input/Actions/IA_ScrollPropSelection`
  (params (ActionValue :type "Float (double-precision)") (ElapsedSeconds :type "Float (double-precision)") (TriggeredSeconds :type "Float (double-precision)") (InputAction :type "InputAction Object Reference" :default "/Game/PropHunt/Input/Actions/IA_ScrollPropSelection.IA_ScrollPropSelection"))
  (:`Triggered`
    (set `self.PropSelection` (+ (`self.PropSelection`) (`KismetMathLibrary.SignOfFloat` ActionValue)))))

(event `HighlightPotentialMesh`
  (bind _currentlyhighlighted (`self.CurrentlyHighlighted`))
  (if (`self.IsLocallyControlled`)
    (bind _asstatic_mesh_component (`self.GetPotentialMesh`)
      (:`true`
        (if (not (== _asstatic_mesh_component (`self.CurrentlyHighlighted`)))
          (`|ExecutionSequence`
            (:`then_0`
              (`/Engine/EditorBlueprintResources/StandardMacros.IsValid` _currentlyhighlighted :!label _label_2
                (:`Is Valid`
                  (`MeshComponent.SetOverlayMaterial` _currentlyhighlighted null false 0)
                  (set `self.CurrentlyHighlighted` null))))
            (:`then_1`
              (bind _output_get (set `self.CurrentlyHighlighted` _asstatic_mesh_component))
              (`MeshComponent.SetOverlayMaterial` _output_get (`self.HighlightMaterial`) false 0)))))
      (:`false`
        (goto _label_2)))))

(fn `UserConstructionScript`)