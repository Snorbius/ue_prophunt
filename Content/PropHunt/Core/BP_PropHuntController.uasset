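; BP_PropHuntController is the Prop Hunt player controller, handling input, ready-up, match start and pausing.
; On local BeginPlay it waits briefly, adds the input mapping, then caches player state, game mode, game state and HUD.
; Tapping ready toggles it via server RPC, while holding attempts game start on authority; O forces it.
; Pause switches input mode; pawn-swap inputs are unwired, though its server event remains.
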(event `SetInputEnabled`
  (params (Value :type Boolean))
  (bind _returnvalue (subsystem `EnhancedInputLocalPlayerSubsystem`))
  (if Value
    (`EnhancedInputSubsystemInterface.AddMappingContext` _returnvalue "/Game/PropHunt/Input/IMC_PropHunt.IMC_PropHunt" 0 (struct))
    (else
      (`EnhancedInputSubsystemInterface.RemoveMappingContext` _returnvalue "/Game/PropHunt/Input/IMC_PropHunt.IMC_PropHunt" (struct)))))

(event `self.ReceiveBeginPlay`
  (if (`self.IsLocalController`)
    (`KismetSystemLibrary.Delay` 1.0)
    (`self.SetInputEnabled` true)
    (bind _asbp_prop_hunt_player_state (cast `/Game/PropHunt/Core/BP_PropHuntPlayerState` (`self.PlayerState`)))
    (set `self.PlayerStateRef` _asbp_prop_hunt_player_state)
    (bind _asgm_prop_hunt (cast `/Game/PropHunt/Core/GM_PropHunt` (`GameplayStatics.GetGameMode`))
      (:`then`
        (set `self.GameModeRef` _asgm_prop_hunt))
      (:`CastFailed`
        _))
    (bind _asbp_prop_hunt_game_state (cast `/Game/PropHunt/Core/BP_PropHuntGameState` (`GameplayStatics.GetGameState`)))
    (set `self.GameStateRef` _asbp_prop_hunt_game_state)
    (bind _asbp_player_hud (cast `/Game/PropHunt/Core/BP_PlayerHud` (`self.GetHUD`)))
    (set `self.HudRef` _asbp_player_hud)))

(event `EnhancedInput|/Game/PropHunt/Input/Actions/IA_SwapToSpectator`
  (params (ActionValue :type Boolean) (ElapsedSeconds :type "Float (double-precision)") (TriggeredSeconds :type "Float (double-precision)") (InputAction :type "InputAction Object Reference" :default "/Game/PropHunt/Input/Actions/IA_SwapToSpectator.IA_SwapToSpectator")))

(event `EnhancedInput|/Game/PropHunt/Input/Actions/IA_SwapToHider`
  (params (ActionValue :type Boolean) (ElapsedSeconds :type "Float (double-precision)") (TriggeredSeconds :type "Float (double-precision)") (InputAction :type "InputAction Object Reference" :default "/Game/PropHunt/Input/Actions/IA_SwapToHider.IA_SwapToHider")))

(event `EnhancedInput|/Game/PropHunt/Input/Actions/IA_SwapToHunter`
  (params (ActionValue :type Boolean) (ElapsedSeconds :type "Float (double-precision)") (TriggeredSeconds :type "Float (double-precision)") (InputAction :type "InputAction Object Reference" :default "/Game/PropHunt/Input/Actions/IA_SwapToHunter.IA_SwapToHunter")))

(event `Server_SwapPlayerType`
  (params (Type :type "/Game/PropHunt/Data/Enums/E_PlayerTypes Enum" :default "NewEnumerator0"))
  (bind _asbp_prop_hunt_player_state (cast `/Game/PropHunt/Core/BP_PropHuntPlayerState` (`self.PlayerState`)))
  (`/Game/PropHunt/Core/BP_PropHuntPlayerState.SwapControlledPawn` _asbp_prop_hunt_player_state Type))

(event `EnhancedInput|/Game/PropHunt/Input/Actions/IA_ToggleReady`
  (params (ActionValue :type Boolean) (ElapsedSeconds :type "Float (double-precision)") (TriggeredSeconds :type "Float (double-precision)") (InputAction :type "InputAction Object Reference" :default "/Game/PropHunt/Input/Actions/IA_ToggleReady.IA_ToggleReady"))
  (bind _gamestateref (`self.GameStateRef`))
  (:`Triggered`
    (`/Game/PropHunt/Core/BP_PropHuntGameState.IsGameStarted` _gamestateref
      (:`then`)
      (:`else`
        (if (>= ElapsedSeconds (`self.ToggleBeginThreshold`))
          (`/Engine/EditorBlueprintResources/StandardMacros.DoOnce` false :!label _label
            (:`Completed`
              (`/Engine/EditorBlueprintResources/ActorMacros.Switch Has Authority`
                (:`Authority`
                  (`/Game/PropHunt/Core/GM_PropHunt.AttemptBeginGame` (`self.GameModeRef`))))))))))
  (:`Completed`
    (`/Game/PropHunt/Core/BP_PropHuntGameState.IsGameStarted` _gamestateref
      (:`then`)
      (:`else`
        (`|ExecutionSequence`
          (:`then_0`
            (goto _label :!via `Reset`))
          (:`then_1`
            (if (<= ElapsedSeconds (`self.ToggleBeginThreshold`))
              (`self.Server_ToggleReady`))))))))

(event `Key|O`
  (params (Key :type "Key Structure"))
  (:`Pressed`
    (`/Engine/EditorBlueprintResources/ActorMacros.Switch Has Authority`
      (:`Authority`
        (`/Game/PropHunt/Core/GM_PropHunt.BeginGame` (`self.GameModeRef`))))))

(event `Server_ToggleReady`
  (bind _asbp_prop_hunt_player_state (cast `/Game/PropHunt/Core/BP_PropHuntPlayerState` (`self.PlayerState`)))
  (`/Game/PropHunt/Core/BP_PropHuntPlayerState.ToggleReady` _asbp_prop_hunt_player_state))

(event `EnhancedInput|/Game/PropHunt/Input/Actions/IA_Pause`
  (params (ActionValue :type Boolean) (ElapsedSeconds :type "Float (double-precision)") (TriggeredSeconds :type "Float (double-precision)") (InputAction :type "InputAction Object Reference" :default "/Game/PropHunt/Input/Actions/IA_Pause.IA_Pause"))
  (bind _hudref (`self.HudRef`))
  (:`Started`
    (`/Game/PropHunt/Core/BP_PlayerHud.PauseGame` _hudref)
    (`self.SetInputMode` (not (`/Game/PropHunt/Blueprints/UI/WBP_PauseMenu.IsPaused` (`/Game/PropHunt/Core/BP_PlayerHud.PauseMenuRef` _hudref))))))

(event `SetInputMode`
  (params (InGame :type Boolean))
  (if InGame
    (`WidgetBlueprintLibrary.SetInputMode_GameOnly` self)
    (set `self.bShowMouseCursor` false)
    (else
      (`WidgetBlueprintLibrary.SetInputMode_GameAndUIEx` self null)
      (set `self.bShowMouseCursor` true))))

(fn `UserConstructionScript`)