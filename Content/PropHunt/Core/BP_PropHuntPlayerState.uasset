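; Player state for Prop Hunt that tracks a player's ready flag and swaps their controlled pawn.
; Ready changes go through a server event that notifies the game mode, while OnRep broadcasts them; game start resets the flag.
; Pawn swapping looks up an enum-to-class map, spawns at the current pawn's transform, destroys it and possesses the replacement.
; It also multicasts hider death particles and sets control rotation.
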(event `Multicast_SpawnHiderDeathParticles`
  (params (Location :type "Vector Structure"))
  (`NiagaraFunctionLibrary.SpawnSystemAtLocation` "/Game/PropHunt/Art/Niagara/NS_HiderDeath.NS_HiderDeath" Location))

(event `ToggleReady`
  (`self.Server_SetReadyState` (not (`self.IsReady`))))

(event `SetControlRotation`
  (params (NewRotation :type "Rotator Structure (by ref)"))
  (`Controller.SetControlRotation` (`self.GetPlayerController`) NewRotation))

(event `self.ReceiveBeginPlay`
  (bind _asbp_prop_hunt_game_state (cast `/Game/PropHunt/Core/BP_PropHuntGameState` (`GameplayStatics.GetGameState`)))
  (add `/Game/PropHunt/Core/BP_PropHuntGameState.OnGameStart` _asbp_prop_hunt_game_state (delegate `ResetReadyState`)))

(event `ResetReadyState`
  (`self.Server_SetReadyState` false))

(event `Server_SetReadyState`
  (params (Value :type Boolean))
  (set `self.IsReady` Value)
  (bind _asgm_prop_hunt (cast `/Game/PropHunt/Core/GM_PropHunt` (`GameplayStatics.GetGameMode`)))
  (`/Game/PropHunt/Core/GM_PropHunt.CheckReadyState` _asgm_prop_hunt))

(fn `OnRep_IsReady`
  (`self.OnReadyStateChanged` (`self.IsReady`))
  (`KismetSystemLibrary.PrintString` "Ready state changed"))

(fn `SwapControlledPawn`
  (params (Enumerator :type "/Game/PropHunt/Data/Enums/E_PlayerTypes Enum" :default "NewEnumerator0"))
  (bind (_value _returnvalue) (`BlueprintMapLibrary.Map_Find` (`self.PlayerCharacterMap`) Enumerator))
  (bind _returnvalue_2 (`Controller.K2_GetPawn` (`self.GetPlayerController`)))
  (bind (_returnvalue_location _returnvalue_rotation) (`KismetMathLibrary.BreakTransform` (`self.GetTransform` _returnvalue_2)))
  (`|ExecutionSequence`
    (:`then_0`
      (`KismetSystemLibrary.PrintText` (`|FormatText` "Changing to {type}" (`|GetEnumeratorNameAsString` Enumerator)))
      (if _returnvalue
        (bind _returnvalue_3 (`|SpawnActorFromClass` _value (`KismetMathLibrary.MakeTransform` _returnvalue_location _returnvalue_rotation) "AlwaysSpawn" "MultiplyWithRoot" null null))
        (`self.K2_DestroyActor` _returnvalue_2)
        (`Controller.Possess` (`self.GetPlayerController`) _returnvalue_3)))))

(fn `UserConstructionScript`)