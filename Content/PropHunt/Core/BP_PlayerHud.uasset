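; Player HUD for PropHunt that creates and drives the main UI, round UI and pause menu widgets.
; On BeginPlay it adds all three to the viewport with the round UI hidden, then binds to BP_PropHuntGameState events.
; Game start, end and hunter/hider count events update ready text and round UI, keeping the display event-driven.
; PauseGame toggles the pause menu's enabled state.
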(event `BindGameStateEvents`
  (bind _asbp_prop_hunt_game_state (cast `/Game/PropHunt/Core/BP_PropHuntGameState` (`GameplayStatics.GetGameState`)))
  (add `/Game/PropHunt/Core/BP_PropHuntGameState.OnGameStart` _asbp_prop_hunt_game_state (`|CreateDelegate` :!event `OnGameStart`))
  (add `/Game/PropHunt/Core/BP_PropHuntGameState.OnNumHuntersChanged` _asbp_prop_hunt_game_state (`|CreateDelegate` :!event `OnNumHuntersChange`))
  (add `/Game/PropHunt/Core/BP_PropHuntGameState.OnNumHidersChange` _asbp_prop_hunt_game_state (`|CreateDelegate` :!event `OnNumHidersChange`))
  (add `/Game/PropHunt/Core/BP_PropHuntGameState.OnVictory` _asbp_prop_hunt_game_state (`|CreateDelegate` :!event `OnGameEnd`)))

(event `self.ReceiveBeginPlay`
  (`self.CreateUI`)
  (`self.BindGameStateEvents`))

(event `CreateUI`
  (bind _returnvalue (`|CreateWidget` "/Game/PropHunt/Blueprints/UI/WBP_UI.WBP_UI_C"))
  (bind _output_get (set `self.UiRef` _returnvalue))
  (`UserWidget.AddToViewport` _output_get 0)
  (bind _returnvalue_2 (`|CreateWidget` "/Game/PropHunt/Blueprints/UI/WBP_RoundUI.WBP_RoundUI_C"))
  (bind _output_get_2 (set `self.RoundUIRef` _returnvalue_2))
  (`UserWidget.AddToViewport` _output_get_2 0)
  (set `Widget.Visibility` "Hidden" _output_get_2)
  (bind _returnvalue_3 (`|CreateWidget` "/Game/PropHunt/Blueprints/UI/WBP_PauseMenu.WBP_PauseMenu_C"))
  (bind _output_get_3 (set `self.PauseMenuRef` _returnvalue_3))
  (`UserWidget.AddToViewport` _output_get_3 0))

(event `OnGameStart`
  (`/Game/PropHunt/Blueprints/UI/WBP_UI.SetReadyTextVisibility` (`self.UiRef`) false)
  (`/Game/PropHunt/Blueprints/UI/WBP_RoundUI.PlayEntryAnimation` (`self.RoundUIRef`)))

(event `PauseGame`
  (bind _pausemenuref (`self.PauseMenuRef`))
  (bind _returnvalue (not (`/Game/PropHunt/Blueprints/UI/WBP_PauseMenu.IsPaused` _pausemenuref)))
  (`/Game/PropHunt/Blueprints/UI/WBP_PauseMenu.SetEnable` _pausemenuref _returnvalue)
  (if _returnvalue
    _))

(event `OnNumHuntersChange`
  (params (Value :type Integer))
  (`/Game/PropHunt/Blueprints/UI/WBP_RoundUI.UpdateNumHunters` (`self.RoundUIRef`) Value))

(event `OnNumHidersChange`
  (params (Value :type Integer))
  (`/Game/PropHunt/Blueprints/UI/WBP_RoundUI.UpdateNumHiders` (`self.RoundUIRef`) Value))

(event `OnGameEnd`
  (`/Game/PropHunt/Blueprints/UI/WBP_UI.SetReadyTextVisibility` (`self.UiRef`) true)
  (`/Game/PropHunt/Blueprints/UI/WBP_RoundUI.HideUI` (`self.RoundUIRef`)))

(fn `UserConstructionScript`)